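; Health regeneration power-up that heals every SCharacter in the world over a series of power-up ticks.
; Each tick gathers all SCharacter actors and calls Heal with HealAmt on those with a valid SHealthComponent, regardless of who triggered it.
; The static mesh and its children hide while the power-up is active, and the actor destroys itself on expiry.
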(event EventOnPowerUpTicked
  (bind _outactors (Actor|GetAllActorsOfClass "/Script/PuzzlePlatforms.SCharacter"))
  (for _array_element _outactors
    (Utilities|IsValid (Actor|GetComponentbyClass _array_element "/Script/PuzzlePlatforms.SHealthComponent")
      (:Is%20Valid
        (Class|SHealthComponent|Heal (Actor|GetComponentbyClass _array_element "/Script/PuzzlePlatforms.SHealthComponent") (Variables|Default|GetHealAmt))))))

(event EventOnPowerUpStateChanged
  (params (bNewIsActive :type Boolean))
  (Rendering|SetVisibility (Variables|Default|GetStaticMesh) (not bNewIsActive) true))

(event EventOnExpired
  (Actor|DestroyActor))

(fn ConstructionScript)