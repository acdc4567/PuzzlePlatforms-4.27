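; Super speed power-up that temporarily doubles the walk speed of the actor that activates it.
; OnActivated stores that actor, hides the pickup mesh and sets its CharacterMovementComponent's MaxWalkSpeed to twice the current GetMaxSpeed.
; OnExpired sets it to half the current GetMaxSpeed and destroys the power-up, both only if the stored actor is still valid.
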(event EventOnExpired
  (bind _other_actorxz1 (Variables|Default|GetOther%20Actorxz1))
  (bind _returnvalue (Actor|GetComponentbyClass _other_actorxz1 "/Script/Engine.CharacterMovementComponent"))
  (Utilities|IsValid _other_actorxz1
    (:Is%20Valid
      (Variables|/Script/Engine.CharacterMovementComponent|SetMaxWalkSpeed _returnvalue (/ (Class|MovementComponent|GetMaxSpeed _returnvalue) 2.0))
      (Actor|DestroyActor))))

(event EventOnActivated
  (params (OtherActorx1 :type Actor%20Object%20Reference))
  (bind _returnvalue (Actor|GetComponentbyClass OtherActorx1 "/Script/Engine.CharacterMovementComponent"))
  (Variables|Default|SetOther%20Actorxz1 OtherActorx1)
  (Rendering|SetVisibility (Variables|Default|GetStaticMesh) false true)
  (Variables|/Script/Engine.CharacterMovementComponent|SetMaxWalkSpeed _returnvalue (* (Class|MovementComponent|GetMaxSpeed _returnvalue) 2.0)))

(fn ConstructionScript)